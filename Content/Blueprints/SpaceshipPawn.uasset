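; Player-controlled spaceship pawn that flies a physics-driven cylinder with boost, roll and pitch input.
; Boost input toggles thruster particles and scales thrust by a curve over time since the press.
; Tick rotates the cylinder locally, mapping roll to yaw, and applies mass-independent force along its up vector.
; Mouse look turns the controller; the ApplyForceToAxis local-space force helper is unused in these graphs.
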(event EventBeginPlay)

(event Collision|EventActorBeginOverlap
  (params (OtherActor :type Actor%20Object%20Reference)))

(event EventTick
  (params (DeltaSeconds :type Float%20%28single-precision%29))
  (bind _cylinder (Variables|Default|GetCylinder))
  (Transformation|AddLocalRotation _cylinder (Math|Rotator|MakeRotator 0.0 (* DeltaSeconds (Variables|Default|GetShipPitchPerSecond)) (* DeltaSeconds (Variables|Default|GetShipRollPerSecond))) false false)
  (Physics|AddForce _cylinder (* (Math|Vector|GetUpVector _cylinder) (Variables|Default|GetShipThrust)) "None" true))

(event Input|ActionEvents|InputActionBoost
  (params (Key :type Key%20Structure))
  (bind _bumthrusterfire (Variables|Default|GetBumThrusterFire))
  (:Pressed
    (Variables|Default|SetShipThrustStartTime (Utilities|Time|GetTimeSeconds))
    ;[1 1 1] Toggle Thruster Fire Particles
    (Components|Activation|SetActive _bumthrusterfire true false))
  (:Released
    (Components|Activation|SetActive _bumthrusterfire false false)))

(event Input|AxisEvents|InputAxisBoost
  (params (AxisValue :type Float%20%28single-precision%29))
  (Variables|Default|SetShipThrust (* 9.8e+02 4.0 AxisValue (Math|Curves|GetFloatValue (Variables|Default|GetShipThrustCurve) (- (Utilities|Time|GetTimeSeconds) (Variables|Default|GetShipThrustStartTime))))))

(event Input|AxisEvents|InputAxisPitch
  (params (AxisValue :type Float%20%28single-precision%29))
  (Variables|Default|SetShipPitchPerSecond (* AxisValue 4e+01)))

(event Input|AxisEvents|InputAxisCameraLookX
  (params (AxisValue :type Float%20%28single-precision%29))
  ;[1 1 1] Mouse Look
  (Pawn|Input|AddControllerYawInput (* AxisValue 45.0 (Utilities|Time|GetWorldDeltaSeconds))))

(event Input|AxisEvents|InputAxisCameraLookY
  (params (AxisValue :type Float%20%28single-precision%29))
  ;[1 1 1] Mouse Look
  (Pawn|Input|AddControllerPitchInput (* AxisValue -45.0 (Utilities|Time|GetWorldDeltaSeconds))))

(event Input|AxisEvents|InputAxisRoll
  (params (AxisValue :type Float%20%28single-precision%29))
  (Variables|Default|SetShipRollPerSecond (* AxisValue 4e+01)))

(fn ConstructionScript)

(fn ApplyForcetoAxis
  (params (ForceVector :type Vector))
  (bind _cylinder (Variables|Default|GetCylinder))
  (Physics|AddForce _cylinder (Math|Vector|RotateVector ForceVector (Transformation|GetWorldRotation _cylinder)) "None" true))